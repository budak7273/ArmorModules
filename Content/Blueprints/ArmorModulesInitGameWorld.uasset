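; Game world init module for the ArmorModules mod that broadcasts ADA messages when schematics are purchased.
; At post-initialization it binds to the purchased-schematic delegate and looks each schematic up in a Messages map.
; On a match, unless the SuppressADA debugging config is set, it messages all players and grants the debug armor modules schematic flagged as cheat access.
; An unconnected loop adding resource sink schematics to the all-schematics list never runs.
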(event `self.K2_OnLifecycleEvent`
  (params (Phase :type "ELifecyclePhase Enum" :default "CONSTRUCTION"))
  (switch `ELifecyclePhase` Phase
    (:`CONSTRUCTION`
      (`/ArmorModules/Blueprints/Lib/PSM_Blueprint_Library.Shipping Safe Log` "PSM Construct"))
    (:`INITIALIZATION`
      (`/ArmorModules/Blueprints/Lib/PSM_Blueprint_Library.Shipping Safe Log` "PSM Init"))
    (:`POST_INITIALIZATION`
      (`/ArmorModules/Blueprints/Lib/PSM_Blueprint_Library.Shipping Safe Log` "PSM PostInit")
      (add `FGSchematicManager.PurchasedSchematicDelegate` (`FGSchematicManager.Get` self) (delegate `OnSchematic`))
      (`/ArmorModules/Blueprints/Lib/PSM_Blueprint_Library.Shipping Safe Log` "SchemMsg bound" "NewEnumerator5"))))

(event `OnSchematic`
  (params (purchasedSchematic :type "FGSchematic Class Reference"))
  (bind (_value _returnvalue) (`BlueprintMapLibrary.Map_Find` (`self.Messages`) purchasedSchematic))
  (`/ArmorModules/Blueprints/Lib/PSM_Blueprint_Library.Shipping Safe Log` "SchemMsg fired" "NewEnumerator5")
  (if _returnvalue
    (if (`ConfigPropertyBool.Value` (cast `/SML/ModList/Properties/BP_ConfigPropertyBool` (`RuntimeBlueprintFunctionLibrary.Conv_ConfigPropertySectionToConfigProperty` (cast `/SML/ModList/Properties/BP_ConfigPropertySection` (`RuntimeBlueprintFunctionLibrary.Conv_ConfigPropertySectionToConfigProperty` (cast `/SML/ModList/Properties/BP_ConfigPropertySection` (`RuntimeBlueprintFunctionLibrary.Conv_ModConfigurationToConfigProperty` "/ArmorModules/Blueprints/ArmorModules_Configuration.ArmorModules_Configuration_C") :!pure true) "Debugging") :!pure true) "SuppressADA") :!pure true))
      (`/ArmorModules/Blueprints/Lib/PSM_Blueprint_Library.Shipping Safe Log` "ADA message suppressed by config")
      (else
        (`FGGameState.SendMessageToAllPlayers` (cast `FGGameState` (`GameplayStatics.GetGameState`) :!pure true) _value)
        (`FGSchematicManager.GiveAccessToSchematic` (`FGSchematicManager.Get` null) "/ArmorModules/Schematics/Schematic_DebugArmorModules.Schematic_DebugArmorModules_C" true)))))