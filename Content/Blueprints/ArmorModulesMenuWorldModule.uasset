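; Menu world module that reskins the character and gear shown in the menu scene with armor materials.
; On the Post Initialization lifecycle phase it waits one second, then scans skeletal and static mesh actors, matching them by display-name substring.
; "Character" actors get five body material slots replaced, while helmet, hover pack and controller meshes get their first slot replaced.
; Debug logging traces each step, and several disconnected experimental nodes remain.
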(event `self.K2_OnLifecycleEvent`
  (params (Phase :type "ELifecyclePhase Enum" :default "CONSTRUCTION"))
  (`/ArmorModules/Blueprints/Lib/PSM_Blueprint_Library.Shipping Safe Log` (`KismetStringLibrary.Concat_StrStr` "MenuWorld lifecycle phase: " (`|GetEnumeratorNameAsString` Phase)))
  (switch `ELifecyclePhase` Phase
    (:`POST_INITIALIZATION`
      (`KismetSystemLibrary.Delay` 1.0) ; TODO unsure if needed
      (bind _outactors (`GameplayStatics.GetAllActorsOfClass` "/Script/Engine.SkeletalMeshActor"))
      (`/ArmorModules/Blueprints/Lib/PSM_Blueprint_Library.Shipping Safe Log` (`KismetStringLibrary.Concat_StrStr` "Found N items: " (`KismetStringLibrary.Conv_IntToString` (`KismetArrayLibrary.Array_Length` _outactors))))
      (for _array_element _outactors
        (`/ArmorModules/Blueprints/Lib/PSM_Blueprint_Library.Shipping Safe Log` (`KismetStringLibrary.Concat_StrStr` "Found skeletal mesh: " (`KismetSystemLibrary.GetDisplayName` _array_element)))
        (if (`KismetStringLibrary.Contains` (`KismetSystemLibrary.GetDisplayName` _array_element) "Character")
          (bind _skeletalmeshcomponent (`SkeletalMeshActor.SkeletalMeshComponent` _array_element))
          (for (_array_element_2 _array_index) (`MeshComponent.GetMaterials` _skeletalmeshcomponent)
            (`/ArmorModules/Blueprints/Lib/PSM_Blueprint_Library.Shipping Safe Log` (`KismetStringLibrary.Concat_StrStr` "Material index " (`KismetStringLibrary.Conv_IntToString` _array_index) " is " (`KismetSystemLibrary.GetDisplayName` _array_element_2))))
          (`PrimitiveComponent.SetMaterial` _skeletalmeshcomponent 0 (`self.Body2`))
          (`PrimitiveComponent.SetMaterial` _skeletalmeshcomponent 1 (`self.Body1`))
          (`PrimitiveComponent.SetMaterial` _skeletalmeshcomponent 2 (`self.BodyDetail`))
          (`PrimitiveComponent.SetMaterial` _skeletalmeshcomponent 3 (`self.Hands`))
          (`PrimitiveComponent.SetMaterial` _skeletalmeshcomponent 4 (`self.Backpack`))))
      (bind _outactors_2 (`GameplayStatics.GetAllActorsOfClass` "/Script/Engine.StaticMeshActor"))
      (for _array_element_3 _outactors_2
        (`/ArmorModules/Blueprints/Lib/PSM_Blueprint_Library.Shipping Safe Log` (`KismetStringLibrary.Concat_StrStr` "found SM " (`KismetSystemLibrary.GetDisplayName` _array_element_3) " Component is " (`KismetSystemLibrary.GetDisplayName` (`StaticMeshActor.StaticMeshComponent` _array_element_3))))
        (bind _returnvalue (`KismetSystemLibrary.GetDisplayName` _array_element_3))
        (if (`KismetStringLibrary.Contains` _returnvalue "Helmet" true)
          (bind _staticmeshcomponent (`StaticMeshActor.StaticMeshComponent` _array_element_3))
          (`PrimitiveComponent.SetMaterial` _staticmeshcomponent 0 (`self.Helmet`))
          (`/ArmorModules/Blueprints/Lib/PSM_Blueprint_Library.Shipping Safe Log` "Set helmet")
          (elif (and (`KismetStringLibrary.Contains` _returnvalue "HoverPack" true) (not (`KismetStringLibrary.Contains` _returnvalue "Controller" true)))
            (`PrimitiveComponent.SetMaterial` _staticmeshcomponent 0 (`self.HoverPackBack`))
            (`/ArmorModules/Blueprints/Lib/PSM_Blueprint_Library.Shipping Safe Log` "Set hoverpack back")
            (elif (`KismetStringLibrary.Contains` _returnvalue "HoverPackController" true)
              (`PrimitiveComponent.SetMaterial` _staticmeshcomponent 0 (`self.HoverPackController`))
              (`/ArmorModules/Blueprints/Lib/PSM_Blueprint_Library.Shipping Safe Log` "Set hoverpack controller"))))))))