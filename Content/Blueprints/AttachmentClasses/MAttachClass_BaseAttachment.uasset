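; Base class for armor module suit attachments, handling install/uninstall feedback and fuel consumption.
; On owning clients, timestamps and a delayed uninstall timer filter out quick reinstalls and fuse-break reboots before playing config-gated sounds.
; The server caches suit fuel multipliers on stat updates; fuel use passes through an overridable hook, then applies them, adding the flight multiplier while flying, if config enables fuel.
; The fuel requirement in the condition check remains unimplemented.
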(event `self.ReceiveBeginPlay`
  (`parent.ReceiveBeginPlay`)
  (bind _output_get (set `self.Cached Config Does Anything Require Fuel` (`.bSuccess` (cast `/SML/ModList/Properties/BP_ConfigPropertyBool` (`RuntimeBlueprintFunctionLibrary.Conv_ConfigPropertySectionToConfigProperty` (cast `/SML/ModList/Properties/BP_ConfigPropertySection` (`RuntimeBlueprintFunctionLibrary.Conv_ConfigPropertySectionToConfigProperty` (cast `/SML/ModList/Properties/BP_ConfigPropertySection` (`RuntimeBlueprintFunctionLibrary.Conv_ModConfigurationToConfigProperty` "/ArmorModules/ArmorModules_Configuration.ArmorModules_Configuration_C") :!pure true) "Balance") :!pure true) "ModulesConsumeFuel") :!pure true))))
  (`/ArmorModules/Blueprints/Lib/PSM_Blueprint_Library.Shipping Safe Log` (`KismetStringLibrary.Concat_StrStr` "Config anything requires fuel: " (`KismetStringLibrary.Conv_BoolToString` _output_get)) "NewEnumerator3"))

(event `self.AttachmentInstalled`
  (params (Item :type "InventoryItem Structure"))
  (bind _parentmodule (`self.ParentModule`))
  (bind _powermodule (`EquipmentModuleComponent.PowerModule` _parentmodule))
  (bind _returnvalue (`EMC_PowerModule.GetOverDrawDuration` _powermodule))
  (bind _returnvalue_2 (`EMC_PowerModule.GetFuseTimerDuration` _powermodule))
  (bind _returnvalue_3 (`KismetMathLibrary.FTrunc` (+ (* (+ _returnvalue_2 _returnvalue) 1000.0) 1000.0)))
  (bind _is_within_ (`/ArmorModules/Blueprints/Lib/PSM_Blueprint_Library.Date Time Within N Milliseconds Of Now` (`EquipmentModuleComponent.nFuseBreakOverDraw` _parentmodule) _returnvalue_3))
  (`parent.AttachmentInstalled` Item)
  (`/Engine/EditorBlueprintResources/ActorMacros.Switch Has Authority`
    (:`Authority`
      (add `PowerSuit.OnPowerSuitStatUpdate` (`EquipmentModuleComponent.EquipmentParent` (`self.ParentModule`)) (delegate `OnPowerSuitStatUpdate`)))
    (:`Remote`
      _))
  (if (`FGBlueprintFunctionLibrary.IsLocallyHumanControlled` (`self.GetInstigator`))
    (`/ArmorModules/Blueprints/Lib/PSM_Blueprint_Library.Shipping Safe Log` (`KismetStringLibrary.Concat_StrStr` "Attachment spawned from module in slot " (`KismetStringLibrary.Conv_IntToString` (`self.InventorySlot`)) ": " (`/ArmorModules/Blueprints/Lib/PSM_Blueprint_Library.Get Module Name from Item` Item)) "NewEnumerator2")
    (if (`/ArmorModules/Blueprints/Lib/PSM_Blueprint_Library.Date Time Within N Milliseconds Of Now` (`self._LastUninstalled`) 100)
      (`/ArmorModules/Blueprints/Lib/PSM_Blueprint_Library.Shipping Safe Log` "Was within N of now so reinstall (killing timer)")
      (`KismetSystemLibrary.K2_ClearAndInvalidateTimerHandle` (stale `self.AttachmentUnInstalled` _returnvalue_2) :!label _label)
      (else
        (`/ArmorModules/Blueprints/Lib/PSM_Blueprint_Library.Shipping Safe Log` (`KismetStringLibrary.Concat_StrStr` "Suit fuse timer is " (`KismetStringLibrary.Concat_StrStr` (`KismetStringLibrary.Conv_DoubleToString` _returnvalue_2) "seconds and overdraw is " (`KismetStringLibrary.Conv_DoubleToString` _returnvalue)) "seconds, which means MS is " (`KismetStringLibrary.Conv_IntToString` _returnvalue_3) ". The fuse timer was at " (`/ArmorModules/Blueprints/Lib/PSM_Blueprint_Library.DateTime to Timestamp String` (`EquipmentModuleComponent.nFuseBreakOverDraw` (`self.ParentModule`))) " and Now is " (`/ArmorModules/Blueprints/Lib/PSM_Blueprint_Library.DateTime to Timestamp String` (`KismetMathLibrary.Now`)) " which is within?:  " (`KismetStringLibrary.Conv_BoolToString` _is_within_)))
        (if _is_within_
          (`/ArmorModules/Blueprints/Lib/PSM_Blueprint_Library.Shipping Safe Log` "Was within suit reboot timeframe, so reinstall (killing timer)")
          (goto _label)
          (else
            (`/ArmorModules/Blueprints/Lib/PSM_Blueprint_Library.Shipping Safe Log` "Was not a reinstall and not a reboot, so calling fresh install")
            (`self.Fresh Install` Item)))))))

(event `OnPowerSuitStatUpdate`
  (params (Type :type Integer))
  ;[1 1 1] TODO filter to only certain types?
  (bind _output_get (set `self.CachedSuitFuelConsumptionMult` (+ (`.Multiplier` (break `ModMultProperty` (`EquipmentModuleComponent.GetNamedPropertySafe` (`self.ParentModule`) (`/ArmorModules/Blueprints/Lib/PSM_Blueprint_Library.Get Name of Custom Property` "NewEnumerator2")))) 1.0)))
  (bind _output_get_2 (set `self.CachedSuitFlightFuelConsumptionMult` (+ (`.Multiplier` (break `ModMultProperty` (`EquipmentModuleComponent.GetNamedPropertySafe` (`self.ParentModule`) (`/ArmorModules/Blueprints/Lib/PSM_Blueprint_Library.Get Name of Custom Property` "NewEnumerator3")))) 1.0)))
  (`/ArmorModules/Blueprints/Lib/PSM_Blueprint_Library.Shipping Safe Log` (`KismetStringLibrary.Concat_StrStr` (`KismetSystemLibrary.GetDisplayName` self) ": Cached fuel consumption mult is now: " (`KismetStringLibrary.Conv_DoubleToString` _output_get) "  Cached flight specific fuel consumption mult is now: " (`KismetStringLibrary.Conv_DoubleToString` _output_get_2)) "NewEnumerator3"))

(event `self.AttachmentUnInstalled`
  (bind _asfgcharacter_player (`/ArmorModules/Blueprints/Lib/PSM_Blueprint_Library.Get MAttach Wearing Player` (`self.ParentModule`)))
  (bind _nfusebreakoverdraw (`EquipmentModuleComponent.nFuseBreakOverDraw` (`self.ParentModule`)))
  (bind _returnvalue (`KismetStringLibrary.Concat_StrStr` "Last FuseBreakOverDraw event was " (`/ArmorModules/Blueprints/Lib/PSM_Blueprint_Library.DateTime to Timestamp String` _nfusebreakoverdraw) "  and Now is " (`/ArmorModules/Blueprints/Lib/PSM_Blueprint_Library.DateTime to Timestamp String` (`KismetMathLibrary.Now`))))
  (`parent.AttachmentUnInstalled`)
  (`/Engine/EditorBlueprintResources/ActorMacros.Switch Has Authority`
    (:`Authority`
      (remove `PowerSuit.OnPowerSuitStatUpdate` (`EquipmentModuleComponent.EquipmentParent` (`self.ParentModule`)) (delegate `OnPowerSuitStatUpdate`)))
    (:`Remote`
      _))
  (if (`FGBlueprintFunctionLibrary.IsLocallyHumanControlled` (`self.GetInstigator`))
    (set `self.Cached Wearing Player` _asfgcharacter_player)
    (`/ArmorModules/Blueprints/Lib/PSM_Blueprint_Library.Shipping Safe Log` (`KismetStringLibrary.Concat_StrStr` "Uninstalling attachment in slot " (`KismetStringLibrary.Conv_IntToString` (`self.InventorySlot`)) "  Wearing player is " (`KismetSystemLibrary.GetDisplayName` _asfgcharacter_player)) "NewEnumerator2")
    (set `self._LastUninstalled` (`KismetMathLibrary.Now`))
    (if (`/ArmorModules/Blueprints/Lib/PSM_Blueprint_Library.Date Time Within N Milliseconds Of Now` _nfusebreakoverdraw (`KismetMathLibrary.FTrunc` (+ (* (`EMC_PowerModule.GetOverDrawDuration` (`EquipmentModuleComponent.PowerModule` (`self.ParentModule`))) 1000.0) 1000.0)))
      (`/ArmorModules/Blueprints/Lib/PSM_Blueprint_Library.Shipping Safe Log` (`KismetStringLibrary.Concat_StrStr` "Fuse broke recently, so not considering this a real uninstall. " _returnvalue))
      (else
        (`/ArmorModules/Blueprints/Lib/PSM_Blueprint_Library.Shipping Safe Log` (`KismetStringLibrary.Concat_StrStr` "Starting uninstall timer. " _returnvalue))
        (bind _returnvalue_2 (`KismetSystemLibrary.K2_SetTimerDelegate` (delegate `UninstalledRanOut`) 0.5)) ; Create a timer to wear off\nIf we get installed again,\nthe timer will be killed,\nand unequip won't play
      ))))

(event `UninstalledRanOut`
  (bind _cached_wearing_player (`self.Cached Wearing Player`))
  (`/ArmorModules/Blueprints/Lib/PSM_Blueprint_Library.Shipping Safe Log` (`KismetStringLibrary.Concat_StrStr` "Cached wearing is valid?: " (`KismetStringLibrary.Conv_BoolToString` (`KismetSystemLibrary.IsValid` _cached_wearing_player))))
  (`self.Actually Uninstalled` (not (`FGCharacterBase.IsAliveAndWell` _cached_wearing_player)))
  ;[1 1 1] TODO implement this. Should be fine to call it here, but need to be sure uninstall logic works
  (if (`self.Safe to Destroy on Uninstall`)
    (`/ArmorModules/Blueprints/Lib/PSM_Blueprint_Library.Shipping Safe Log` "Attach was marked safe to destroy so killing it")
    (`self.K2_DestroyActor`)))

(fn `Actually Uninstalled`
  (params (IsPlayerSuspectedDead :type Boolean :default false))
  (`/ArmorModules/Blueprints/Lib/PSM_Blueprint_Library.Shipping Safe Log` (`KismetStringLibrary.Concat_StrStr` "Actually unequipped timer ran out. Suspected dead: " (`KismetStringLibrary.Conv_BoolToString` IsPlayerSuspectedDead)))
  (if IsPlayerSuspectedDead
    ;[1 1 1] TODO does not seem to work yet. Seems like can't play sound after death. Not sure why this is breaking now, worked fine before. Is using cached player so it's not like the player is invalid
    (if (== (`KismetMathLibrary.RandomIntegerInRange` 0 100) 0)
      (`self.ModulePlaySound` null "/ArmorModules/Assets/Audio/RefillEquipSoundConcurrency.RefillEquipSoundConcurrency"))
    (else
      (`self.ModulePlaySound` (`self.Uninstall Sound`) "/ArmorModules/Assets/Audio/RefillEquipSoundConcurrency.RefillEquipSoundConcurrency" 1.0 (`self.(Un)Install sound Category`)))))

(fn `ArmorModules Get Delta Fuel Consumption`
  (params (`Delta Time` :type "Float (double-precision)") (`PreCalc'd Fuel Consumption` :type "Float (double-precision)"))
  (returns (DeltaTime_ :type "Float (double-precision)") (`Fuel Consumption` :type "Float (double-precision)"))
  (return `Delta Time` `PreCalc'd Fuel Consumption`))

(fn `Display Chat Message to Wearer`
  (params (Message :type String))
  (bind _asfgplayer_controller (cast `FGPlayerController` (`Pawn.GetController` (`/ArmorModules/Blueprints/Lib/PSM_Blueprint_Library.Get MAttach Wearing Player` (`self.ParentModule`)))))
  (`/ArmorModules/Blueprints/Lib/PSM_Blueprint_Library.Shipping Safe Log` Message)
  (`FGPlayerController.EnterChatMessage` _asfgplayer_controller Message))

(fn `Fresh Install`
  (params (Item :type "InventoryItem Structure"))
  (`/ArmorModules/Blueprints/Lib/PSM_Blueprint_Library.Shipping Safe Log` "Was NOT within N of now so was fresh installed" "NewEnumerator3")
  (`self.ModulePlaySound` (`self.Install Sound`) "/ArmorModules/Assets/Audio/RefillEquipSoundConcurrency.RefillEquipSoundConcurrency" 1.0 (`self.(Un)Install sound Category`)))

(fn `Get Inventory Slot Index For Widgets`
  (returns (InventorySlotIndex :type Integer))
  (return (`self.InventorySlot`)))

(fn `GetDeltaFuelConsumption`
  (params (DeltaTime :type "Float (double-precision)"))
  (returns (ReturnValue :type "Float (double-precision)"))
  (bind _returnvalue (`parent.GetDeltaFuelConsumption` DeltaTime))
  (if (`self.Cached Config Does Anything Require Fuel`)
    (bind (_deltatime_ _fuel_consumption) (`self.ArmorModules Get Delta Fuel Consumption` DeltaTime _returnvalue))
    (if (> _fuel_consumption 0.0)
      (return (`/ArmorModules/Blueprints/Lib/PSM_Blueprint_Library.Get Fuel Consumption Factoring In Multiplier` _fuel_consumption (+ (`KismetMathLibrary.SelectFloat` (`self.CachedSuitFlightFuelConsumptionMult`) 0.0 (`/ArmorModules/Blueprints/Lib/PSM_Blueprint_Library.Is Flight Related Movement State?` (`EquipmentModuleComponent.SuitState` (`self.ParentModule`)))) (`self.CachedSuitFuelConsumptionMult`))))
      (else
        (return 0.0)))
    (else
      (return 0.0))))

(fn `GetIsConditionMet`
  (returns (ReturnValue :type Boolean))
  (if (`self.ShouldDeactivate`)
    (return false) ; Module itself wants to be turned off
    (elif (`self.Requires Fuel to Operate`)
      (if (`self.bIsActive`)
        (return true) ; TODO implement fuel requried to operate somehow
        (else
          (return true) ; TODO implement fuel requried to operate somehow
        ))
      (else
        (return true) ; No need to check fuel
      ))))

(fn `ModulePlaySound`
  (params (`Sound Base` :type "SoundBase Object Reference") (`Concurrency Settings` :type "SoundConcurrency Object Reference") (`Pitch Multiplier` :type "Float (double-precision)" :default 1.0) (Category :type "/ArmorModules/Blueprints/Lib/ArmorModules_SoundCategories Enum" :default "NewEnumerator0"))
  (bind _returnvalue (* (`/ArmorModules/Blueprints/Lib/PSM_Blueprint_Library.Get Volume for Category` "NewEnumerator0") (`/ArmorModules/Blueprints/Lib/PSM_Blueprint_Library.Get Volume for Category` Category)))
  (if (`FGBlueprintFunctionLibrary.IsLocallyHumanControlled` (`self.GetInstigator`))
    (if (`.bSuccess` (cast `/SML/ModList/Properties/BP_ConfigPropertyBool` (`RuntimeBlueprintFunctionLibrary.Conv_ConfigPropertySectionToConfigProperty` (cast `/SML/ModList/Properties/BP_ConfigPropertySection` (`RuntimeBlueprintFunctionLibrary.Conv_ConfigPropertySectionToConfigProperty` (cast `/SML/ModList/Properties/BP_ConfigPropertySection` (`RuntimeBlueprintFunctionLibrary.Conv_ModConfigurationToConfigProperty` "/ArmorModules/ArmorModules_Configuration.ArmorModules_Configuration_C") :!pure true) "Sounds") :!pure true) "SoundsEnabled") :!pure true))
      (`/Engine/EditorBlueprintResources/StandardMacros.IsValid` `Sound Base`
        (:`Is Valid`
          (`GameplayStatics.PlaySound2D` `Sound Base` _returnvalue `Pitch Multiplier` 0.0 `Concurrency Settings` (`self.Cached Wearing Player`))
          (`/ArmorModules/Blueprints/Lib/PSM_Blueprint_Library.Shipping Safe Log` (`KismetStringLibrary.Concat_StrStr` "Playing sound: " (`KismetSystemLibrary.GetDisplayName` `Sound Base`) " at volume: " (`KismetStringLibrary.Conv_DoubleToString` _returnvalue)) "NewEnumerator2"))
        (:`Is Not Valid`
          (`/ArmorModules/Blueprints/Lib/PSM_Blueprint_Library.Shipping Safe Log` (`KismetStringLibrary.Concat_StrStr` "Sound was not valid: " (`KismetSystemLibrary.GetDisplayName` `Sound Base`)) "NewEnumerator1"))))))

(fn `UserConstructionScript`)