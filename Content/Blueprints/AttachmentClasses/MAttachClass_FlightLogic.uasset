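; Flight logic attachment for armor modules that unlocks suit flight and can force gravity or no-gravity mode on install.
; Flight requires fuel only when both the module and the cached config demand it, gating the condition check and fuel consumption.
; Tick optionally zeroes very low flight velocity and switches the suit to hover.
; Two crouch releases within a configured leeway turn flight off, with multiplayer support noted as uncertain.
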(event `self.AttachmentInstalled`
  (params (Item :type "InventoryItem Structure"))
  (bind _parentmodule (`self.ParentModule`))
  (`parent.AttachmentInstalled` Item)
  (bind _output_get (set `self.CachedConfigFlightFuelRequirement` (`ConfigPropertyBool.Value` (cast `/SML/ModList/Properties/BP_ConfigPropertyBool` (`RuntimeBlueprintFunctionLibrary.Conv_ConfigPropertySectionToConfigProperty` (cast `/SML/ModList/Properties/BP_ConfigPropertySection` (`RuntimeBlueprintFunctionLibrary.Conv_ConfigPropertySectionToConfigProperty` (cast `/SML/ModList/Properties/BP_ConfigPropertySection` (`RuntimeBlueprintFunctionLibrary.Conv_ModConfigurationToConfigProperty` "/ArmorModules/ArmorModules_Configuration.ArmorModules_Configuration_C") :!pure true) "Balance") :!pure true) "FlightRequiresFuel") :!pure true))))
  (`/ArmorModules/Blueprints/Lib/PSM_Blueprint_Library.Shipping Safe Log` (`KismetStringLibrary.Concat_StrStr` "Config is fuel needed for flight?: " (`KismetStringLibrary.Conv_BoolToString` _output_get)))
  (if (`self.ForceNoGravityModeOnEquip`)
    (`/Engine/EditorBlueprintResources/StandardMacros.IsValid` _parentmodule
      (:`Is Valid`
        (set `EquipmentModuleComponent.TKey_NoGravity` true _parentmodule) ; Enter NoGrav mode
        (`/ArmorModules/Blueprints/Lib/PSM_Blueprint_Library.Shipping Safe Log` "Forced to NoGrav mode" "NewEnumerator5")))
    (elif (`self.ForceGravityModeOnEquip`)
      (set `EquipmentModuleComponent.TKey_NoGravity` false _parentmodule) ; Enter Grav mode
      (`/ArmorModules/Blueprints/Lib/PSM_Blueprint_Library.Shipping Safe Log` "Forced to Grav mode" "NewEnumerator5")
      (else
        (`/ArmorModules/Blueprints/Lib/PSM_Blueprint_Library.Shipping Safe Log` "GravMode unchanged by equipped flight module" "NewEnumerator5")))))

(event `self.AttachmentTick`
  (params (DeltaTime :type "Float (single-precision)"))
  (bind _charactermovement (`Character.CharacterMovement` (`/ArmorModules/Blueprints/Lib/PSM_Blueprint_Library.Get MAttach Wearing Player` (`self.ParentModule`))))
  (bind _returnvalue (`KismetMathLibrary.VSize` (`MovementComponent.Velocity` _charactermovement)))
  (`parent.AttachmentTick` DeltaTime)
  (if (`self.StifleLowVelocity`)
    (if (`/ArmorModules/Blueprints/Lib/PSM_Blueprint_Library.Is Flight Related Movement State?` (`EquipmentModuleComponent.SuitState` (`self.ParentModule`)))
      (if (and (< _returnvalue 15.0) (> _returnvalue 0.0))
        (`self.Stifle Velocity` _charactermovement)))))

(event `InputAction|Crouch` :consume false :overrideparent false
  (params (Key :type "Key Structure"))
  (bind _value (`ConfigPropertyInteger.Value` (cast `/SML/ModList/Properties/BP_ConfigPropertyInteger` (`RuntimeBlueprintFunctionLibrary.Conv_ConfigPropertySectionToConfigProperty` (cast `/SML/ModList/Properties/BP_ConfigPropertySection` (`RuntimeBlueprintFunctionLibrary.Conv_ConfigPropertySectionToConfigProperty` (cast `/SML/ModList/Properties/BP_ConfigPropertySection` (`RuntimeBlueprintFunctionLibrary.Conv_ModConfigurationToConfigProperty` "/ArmorModules/ArmorModules_Configuration.ArmorModules_Configuration_C") :!pure true) "General") :!pure true) "MillisecondsLeewayForFlightCancel") :!pure true)))
  ;[1 1 1] Stop Flying keybind, probably needs mp support
  (:`Pressed`
    (`/ArmorModules/Blueprints/Lib/PSM_Blueprint_Library.Shipping Safe Log` "Crouch pressed" "NewEnumerator5"))
  (:`Released`
    (`/ArmorModules/Blueprints/Lib/PSM_Blueprint_Library.Shipping Safe Log` "Crouch released (checking)" "NewEnumerator5")
    (if (`/ArmorModules/Blueprints/Lib/PSM_Blueprint_Library.Date Time Within N Milliseconds Of Now` (`self.CrouchLastPressed`) _value)
      (`/ArmorModules/Blueprints/Lib/PSM_Blueprint_Library.Shipping Safe Log` (`KismetStringLibrary.Concat_StrStr` "Was within timeframe to stop flight, " (`KismetStringLibrary.Concat_StrStr` "Now is " (`/ArmorModules/Blueprints/Lib/PSM_Blueprint_Library.DateTime to Timestamp String` (`KismetMathLibrary.Now`)) " and then is " (`/ArmorModules/Blueprints/Lib/PSM_Blueprint_Library.DateTime to Timestamp String` (`self.CrouchLastPressed`)) "  -- needs within millseconds" (`KismetStringLibrary.Conv_IntToString` _value))) "NewEnumerator5")
      (set `EquipmentModuleComponent.TKey_Fly` false (`self.ParentModule`)))
    (set `self.CrouchLastPressed` (`KismetMathLibrary.Now`))))

(event `self.ReceiveBeginPlay`
  (`parent.ReceiveBeginPlay`)
  (set `self.CrouchLastPressed` (`KismetMathLibrary.Now`)))

(fn `Allowed to Fly (Fuel)`
  (returns (CanFly :type Boolean))
  (bind _parentmodule (`self.ParentModule`))
  (bind _nfuelamount (`EquipmentModuleComponent.nFuelAmount` _parentmodule))
  (if (and (`self.Requires Fuel to Operate`) (`self.CachedConfigFlightFuelRequirement`))
    (`/Engine/EditorBlueprintResources/StandardMacros.IsValid` _parentmodule
      (:`Is Valid`
        (if (> _nfuelamount 0.0)
          (return true)
          (else
            (`/ArmorModules/Blueprints/Lib/PSM_Blueprint_Library.Shipping Safe Log` (`KismetStringLibrary.Concat_StrStr` "Turning off flight because no fuel (is: " (`KismetStringLibrary.Conv_DoubleToString` _nfuelamount) ")") "NewEnumerator5")
            (return false))))
      (:`Is Not Valid`
        (`/ArmorModules/Blueprints/Lib/PSM_Blueprint_Library.Shipping Safe Log` "Not allowed because parent ref not valid")
        (return false)))
    (else
      (return true))))

(fn `ArmorModules Get Delta Fuel Consumption`
  (params (`Delta Time` :type "Float (double-precision)") (`PreCalc'd Fuel Consumption` :type "Float (double-precision)"))
  (returns (DeltaTime_ :type "Float (double-precision)") (`Fuel Consumption` :type "Float (double-precision)"))
  (if (and (`self.Requires Fuel to Operate`) (`self.CachedConfigFlightFuelRequirement`))
    (bind (_deltatime_ _fuel_consumption) (`parent.ArmorModules Get Delta Fuel Consumption` `Delta Time` `PreCalc'd Fuel Consumption`))
    (`/ArmorModules/Blueprints/Lib/PSM_Blueprint_Library.Shipping Safe Log` (`KismetStringLibrary.Concat_StrStr` "Flight Fuel this tick is: " (`KismetStringLibrary.Conv_DoubleToString` _fuel_consumption)) "NewEnumerator5")
    (return _deltatime_ _fuel_consumption)
    (else
      (return `Delta Time` 0.0))))

(fn `GetIsConditionMet`
  (returns (ReturnValue :type Boolean))
  (return (and (`parent.GetIsConditionMet`) (`self.Allowed to Fly (Fuel)`))))

(fn `ReceiveModuleStats`
  (params (DefaultStats :type "EquipmentStats Structure"))
  (returns (ReturnValue :type "EquipmentStats Structure"))
  (locals (Stats :type "EquipmentStats Structure"))
  (bind _returnvalue (`parent.ReceiveModuleStats` DefaultStats))
  (set `local.Stats` _returnvalue)
  (`PowerSuitBPLibrary.SetSuitFlag` (`local.Stats`) "SuitFlag_HasFlightUnlocked" true)
  (return (`local.Stats`)))

(fn `Stifle Velocity`
  (params (`Movement C` :type "MovementComponent Object Reference"))
  (locals (`Old Movement Mode` :type "EPowerSuitState Enum"))
  (bind _parentmodule (`self.ParentModule`))
  (set `MovementComponent.Velocity` (0.0 0.0 0.0) `Movement C`)
  (set `local.Old Movement Mode` (`EquipmentModuleComponent.SuitState` _parentmodule))
  (bind _output_get (set `EquipmentModuleComponent.SuitState` "PS_HOVER" _parentmodule))
  (`/ArmorModules/Blueprints/Lib/PSM_Blueprint_Library.Shipping Safe Log` "Stifled velocity" "NewEnumerator5"))

(fn `UserConstructionScript`
  (`parent.UserConstructionScript`))