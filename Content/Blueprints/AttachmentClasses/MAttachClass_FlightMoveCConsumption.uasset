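; Attachment class for a flight module that adjusts the movement component's walk and sprint speeds.
; Movement mode changes put the module in its enabled state for hovering, flying and slow fall, and in its disabled state for all other listed modes, including flight falling.
; The modification override adds multiplier-scaled walk and sprint modifiers onto the current speeds rather than setting absolute values, then logs the result outside shipping builds.
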(fn `Apply Move C Modification`
  (params (MoveC :type "FGCharacterMovementComponent Object Reference") (`Multiplier for Change to Add to Current Value` :type "Float (double-precision)") (`Enabling (T) or Disabling(F)` :type Boolean))
  (returns (`New Value` :type "Float (double-precision)"))
  (bind _output_get (set `FGCharacterMovementComponent.mMaxSprintSpeed` (+ (* `Multiplier for Change to Add to Current Value` (`self.Sprint Speed Modifier`)) (`FGCharacterMovementComponent.mMaxSprintSpeed` MoveC)) MoveC))
  (bind _output_get_2 (set `CharacterMovementComponent.MaxWalkSpeed` (+ (* `Multiplier for Change to Add to Current Value` (`self.Walk Speed Modifier`)) (`CharacterMovementComponent.MaxWalkSpeed` MoveC)) MoveC))
  (`/ArmorModules/Blueprints/Lib/PSM_Blueprint_Library.Shipping Safe Log` (`KismetStringLibrary.Concat_StrStr` "Walk speed is now " (`KismetStringLibrary.Conv_DoubleToString` _output_get_2) "    sprint speed is now " (`KismetStringLibrary.Conv_DoubleToString` _output_get)) "NewEnumerator3")
  (return _output_get))

(fn `OnMovementModeChange`
  (params (`Previous Movement Mode` :type "EPowerSuitState Enum" :default "PS_NONE") (`New Movement Mode` :type "EPowerSuitState Enum" :default "PS_NONE"))
  (`parent.OnMovementModeChange` `Previous Movement Mode` `New Movement Mode`)
  (switch `EPowerSuitState` `New Movement Mode`
    (:`PS_NONE`
      (`self.Module Disabled State` `New Movement Mode` :!label _label))
    (:`PS_STANDING`
      (goto _label))
    (:`PS_WALKING`
      (goto _label))
    (:`PS_SPRINTING`
      (goto _label))
    (:`PS_HOVER`
      (`self.Module Enabled State` `New Movement Mode` :!label _label_2))
    (:`PS_FLYUP`
      (goto _label_2))
    (:`PS_FLYDOWN`
      (goto _label_2))
    (:`PS_HOVERMOVE`
      (goto _label_2))
    (:`PS_HOVERSPRINT`
      (goto _label_2))
    (:`PS_PIPEHYPER_RIDE`
      (goto _label))
    (:`PS_PIPEHYPER_SPRINT`
      (goto _label))
    (:`PS_FALLING`
      (goto _label))
    (:`PS_SLIDING`
      (goto _label))
    (:`PS_POWERSLIDE`
      (goto _label))
    (:`PS_ZIPLINE`
      (goto _label))
    (:`PS_ZIPLINE_SPRINT`
      (goto _label))
    (:`PS_REBOOTING`
      (goto _label))
    (:`PS_SLOWFALL`
      (goto _label_2))))

(fn `UserConstructionScript`
  (`parent.UserConstructionScript`))