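; Fueled power generator attachment for suit armor modules that produces power from fuel when the suit needs it.
; On authority, each tick targets the suit's draw minus its own output, or missing stored power if configured, with slight overshoot.
; The replicated usage fraction ramps toward that target and feeds the power and fuel consumption overrides, with production reported as negative draw.
; In editor, a debug widget simulates demand and displays usage.
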(event `self.ReceiveBeginPlay`
  ;[1 1 1] In-Editor testing functionality
  (if (`RuntimeBlueprintFunctionLibrary.IsEditor`)
    (bind _returnvalue (`|CreateWidget` "/ArmorModules/Debug/DebugWidget.DebugWidget_C" null self))
    (`UserWidget.AddToViewport` _returnvalue 0)))

(event `self.ReceiveTick`
  (params (DeltaSeconds :type "Float (single-precision)"))
  ;[1 1 1] In-Editor testing functionality
)

(event `self.AttachmentTick`
  (params (DeltaTime :type "Float (single-precision)"))
  (bind _parentmodule (`self.ParentModule`))
  (bind __targetoutputfraction (`self._TargetOutputFraction`))
  (bind __targetoutputfraction_2 (`self._TargetOutputFraction`))
  (bind _parentmodule_2 (`self.ParentModule`))
  (bind _configshouldfilltocapacity (`self.ConfigShouldFillToCapacity`))
  (bind _returnvalue (- (`self._SuitRawPowerDrawMW`) (`self.Calc Attach Power Consumption MW`)))
  (bind _returnvalue_2 (and _configshouldfilltocapacity (< (`PowerSuit.GetCurrentPower` (`EquipmentModuleComponent.EquipmentParent` _parentmodule)) (`EMC_PowerModule.GetPowerCapacity` (`EquipmentModuleComponent.PowerModule` _parentmodule)))))
  (bind _returnvalue_3 (+ (`KismetMathLibrary.SelectFloat` (- (`EMC_PowerModule.GetPowerCapacity` (`EquipmentModuleComponent.PowerModule` _parentmodule_2)) (`PowerSuit.GetCurrentPower` (`EquipmentModuleComponent.EquipmentParent` _parentmodule_2))) (`self._SuitPowerDrawWithoutMeMW`) _returnvalue_2) 5.0))
  (`parent.AttachmentTick` DeltaTime)
  (`/Engine/EditorBlueprintResources/ActorMacros.Switch Has Authority` ; Only perform the power calculation on the server.\nUsageLastFrame is replicated -> client can calc from there
    (:`Authority`
      (bind _output_get (set `self._RampAmount` (* (select `bool` (`RuntimeBlueprintFunctionLibrary.IsEditor`) :`false` DeltaTime :`true` (stale `self.ReceiveTick` DeltaSeconds)) (`self.RampupSpeedMultiplier`))))
      (if (`RuntimeBlueprintFunctionLibrary.IsEditor`)
        ;[1 1 1] In-Editor testing functionality
        (set `self._SuitRawPowerDrawMW` (+ (`Slider.GetValue` (`/ArmorModules/Debug/DebugWidget.Powerdemandslider` (stale `self.ReceiveBeginPlay` _returnvalue))) (`self.Calc Attach Power Consumption MW`)))
        (bind _returnvalue_4 (`KismetStringLibrary.Concat_StrStr` "FuelBurn Tick RampAmnt: " (`KismetStringLibrary.Conv_DoubleToString` _output_get) "    UsageLastFrame: " (`KismetStringLibrary.Conv_DoubleToString` (`self.UsageFraction_LastFrame`)) "    SuitPowerDraw: " (`KismetStringLibrary.Conv_DoubleToString` (`self._SuitRawPowerDrawMW`)) "    Suit Fuel amount: " (`KismetStringLibrary.Conv_DoubleToString` (`EquipmentModuleComponent.nFuelAmount` (`self.ParentModule`)))))
        (`/ArmorModules/Blueprints/Lib/PSM_Blueprint_Library.Shipping Safe Log` _returnvalue_4 "NewEnumerator5")
        (`/ArmorModules/Debug/DebugWidget.Set ProgressBar Display Val` (stale `self.ReceiveBeginPlay` _returnvalue) (`self.UsageFraction_LastFrame`))
        (else
          (set `self._SuitRawPowerDrawMW` (`EMC_PowerModule.GetPowerDraw` (`EquipmentModuleComponent.PowerModule` (`self.ParentModule`))))
          (`/ArmorModules/Blueprints/Lib/PSM_Blueprint_Library.Shipping Safe Log` _returnvalue_4 "NewEnumerator5")))
      (set `self._SuitPowerDrawWithoutMeMW` _returnvalue)
      (`/ArmorModules/Blueprints/Lib/PSM_Blueprint_Library.Shipping Safe Log` (`KismetStringLibrary.Concat_StrStr` "Suit draw after removing me:" (`KismetStringLibrary.Conv_DoubleToString` _returnvalue) "    Config says to turn on whenever not full? " (`KismetStringLibrary.Conv_BoolToString` _configshouldfilltocapacity)) "NewEnumerator5")
      (if (or _returnvalue_2 (> _returnvalue 0.0))
        (bind _output_get_2 (set `self._TargetOutputFraction` (`KismetMathLibrary.FClamp` (/ _returnvalue_3 (`self.PowerOutputMaxMW`)))))
        (`/ArmorModules/Blueprints/Lib/PSM_Blueprint_Library.Shipping Safe Log` (`KismetStringLibrary.Concat_StrStr` "Target MW is " (`KismetStringLibrary.Conv_DoubleToString` _returnvalue_3)))
        (if (`KismetMathLibrary.NearlyEqual_FloatFloat` _output_get_2 (`self.UsageFraction_LastFrame`) 0.01)
          (bind _output_get_3 (set `self.UsageFraction_LastFrame` (`self._TargetOutputFraction`)))
          (`/ArmorModules/Blueprints/Lib/PSM_Blueprint_Library.Shipping Safe Log` (`KismetStringLibrary.Concat_StrStr` "Snap to target which is " (`KismetStringLibrary.Conv_DoubleToString` _output_get_3)) "NewEnumerator5")
          (elif (> (`self.UsageFraction_LastFrame`) (`self._TargetOutputFraction`))
            (bind _output_get_4 (set `self.UsageFraction_LastFrame` (`KismetMathLibrary.FClamp` (- (`self.UsageFraction_LastFrame`) (`self._RampAmount`)) __targetoutputfraction)))
            (`/ArmorModules/Blueprints/Lib/PSM_Blueprint_Library.Shipping Safe Log` (`KismetStringLibrary.Concat_StrStr` "Ramp down to meet, at" (`KismetStringLibrary.Conv_DoubleToString` _output_get_4) ", target is " (`KismetStringLibrary.Conv_DoubleToString` __targetoutputfraction)) "NewEnumerator5")
            (else
              (bind _output_get_5 (set `self.UsageFraction_LastFrame` (`KismetMathLibrary.FClamp` (+ (`self.UsageFraction_LastFrame`) (`self._RampAmount`)) 0.0 __targetoutputfraction_2)))
              (`/ArmorModules/Blueprints/Lib/PSM_Blueprint_Library.Shipping Safe Log` (`KismetStringLibrary.Concat_StrStr` "Ramp up to meet, at " (`KismetStringLibrary.Conv_DoubleToString` _output_get_5) ", target is " (`KismetStringLibrary.Conv_DoubleToString` __targetoutputfraction_2)) "NewEnumerator5"))))
        (else
          (bind _output_get_6 (set `self.UsageFraction_LastFrame` (`KismetMathLibrary.FClamp` (- (`self.UsageFraction_LastFrame`) (`self._RampAmount`))))) ; It isn't - Ramp down to 0 production
          (if (not (`KismetMathLibrary.NearlyEqual_FloatFloat` _output_get_6))
            (`/ArmorModules/Blueprints/Lib/PSM_Blueprint_Library.Shipping Safe Log` (`KismetStringLibrary.Concat_StrStr` "Ramp Down to 0, at " (`KismetStringLibrary.Conv_DoubleToString` _output_get_6)) "NewEnumerator5"))))
      ;[1 1 1] Further editor logging
      (if (`RuntimeBlueprintFunctionLibrary.IsEditor`)
        (if (not (`KismetMathLibrary.NearlyEqual_FloatFloat` (`self.UsageFraction_LastFrame`)))
          (`/ArmorModules/Blueprints/Lib/PSM_Blueprint_Library.Shipping Safe Log` (`KismetStringLibrary.Concat_StrStr` "Module power consumption MW" (`KismetStringLibrary.Conv_DoubleToString` (`self.Calc Attach Power Consumption MW`))) "NewEnumerator1")
          (`/ArmorModules/Blueprints/Lib/PSM_Blueprint_Library.Shipping Safe Log` (`KismetStringLibrary.Concat_StrStr` "Module fuel  consumption MW" (`KismetStringLibrary.Conv_DoubleToString` (`self.Calc Attach Desired Fuel Consumption MW`))) "NewEnumerator1"))))))

(event `self.AttachmentInstalled`
  (params (Item :type "InventoryItem Structure"))
  (`parent.AttachmentInstalled` Item)
  (set `self.ConfigShouldFillToCapacity` (`ConfigPropertyBool.Value` (cast `/SML/ModList/Properties/BP_ConfigPropertyBool` (`RuntimeBlueprintFunctionLibrary.Conv_ConfigPropertySectionToConfigProperty` (cast `/SML/ModList/Properties/BP_ConfigPropertySection` (`RuntimeBlueprintFunctionLibrary.Conv_ModConfigurationToConfigProperty` "/ArmorModules/Blueprints/ArmorModules_Configuration.ArmorModules_Configuration_C") :!pure true) "FueledGenFillCapacity") :!pure true))))

(fn `ArmorModules Get Delta Fuel Consumption`
  (params (`Delta Time` :type "Float (double-precision)") (`PreCalc'd Fuel Consumption` :type "Float (double-precision)"))
  (returns (DeltaTime_ :type "Float (double-precision)") (`Fuel Consumption` :type "Float (double-precision)"))
  (bind _returnvalue (`self.Calc Attach Desired Fuel Consumption MW`))
  (bind (_deltatime_ _fuel_consumption) (`parent.ArmorModules Get Delta Fuel Consumption` `Delta Time` `PreCalc'd Fuel Consumption`))
  (`/ArmorModules/Blueprints/Lib/PSM_Blueprint_Library.Shipping Safe Log` (`KismetStringLibrary.Concat_StrStr` "Pre-Mult Fuel consumption will be " (`KismetStringLibrary.Conv_DoubleToString` _returnvalue)) "NewEnumerator5")
  (return _deltatime_ (+ _fuel_consumption _returnvalue)))

(fn `GetDeltaPowerConsumption`
  (params (DeltaTime :type "Float (double-precision)"))
  (returns (ReturnValue :type "Float (double-precision)"))
  (return (`self.Calc Attach Power Consumption MW`)))

(fn `UserConstructionScript`)