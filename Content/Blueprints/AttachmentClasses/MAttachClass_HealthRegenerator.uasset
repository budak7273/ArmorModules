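; Health regenerator attachment class that sets the module's power draw according to the wearing player's health.
; GetDeltaPowerConsumption returns active consumption while the wearer's MHealthComponent is below max health, otherwise inactive consumption.
; An invalid health component logs a message and falls back to active consumption.
; RecieveModuleStats passes stats through unchanged; its health regen suit modifier is disconnected and marked TODO, so this class applies no healing itself.
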(fn `GetDeltaPowerConsumption`
  (params (DeltaTime :type "Float (double-precision)"))
  (returns (ReturnValue :type "Float (double-precision)"))
  (bind _mhealthcomponent (`FGCharacterBase.mHealthComponent` (`/ArmorModules/Blueprints/Lib/PSM_Blueprint_Library.Get MAttach Wearing Player` (`self.ParentModule`))))
  (`parent.GetDeltaPowerConsumption` DeltaTime)
  (`/Engine/EditorBlueprintResources/StandardMacros.IsValid` _mhealthcomponent
    (:`Is Valid`
      (if (< (`FGHealthComponent.mCurrentHealth` _mhealthcomponent) (`FGHealthComponent.GetMaxHealth` _mhealthcomponent))
        _
        (else
          (return (`self.InactivePowerConsumption`)) ; Idle power consumption
        )))
    (:`Is Not Valid`
      (`/ArmorModules/Blueprints/Lib/PSM_Blueprint_Library.Shipping Safe Log` "HealthRegen somewhere along the way to health component was invalid. Falling back to always on consumption.")))
  (return (`self.ActivePowerConsumption`)) ; Regenerating power consumption
)

(fn `RecieveModuleStats`
  (params (DefaultStats :type "EquipmentStats Structure"))
  (returns (ReturnValue :type "EquipmentStats Structure"))
  (return DefaultStats))

(fn `UserConstructionScript`)