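; Armor module attachment that consumes items from the wearing player's inventory to keep an internal charge buffer filled.
; BeginPlay reads a per-category config toggle, which authority multicasts; with consumption off, authority keeps the buffer full.
; Post-tick, after production is decided, authority refuels an empty buffer from the accepted items, with a refill sound if locally controlled.
; The buffer drains only while the parent module produces, using charge lifetime and drain multiplier.
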(event `ConfigBoolMultiCast`
  (params (ConfigBool :type Boolean))
  ;[1 1 1] Needs testing
  (set `self.ConfigBool` ConfigBool))

(event `self.ReceiveBeginPlay`
  (bind _configitemconsumptioncategory (`self.ConfigItemConsumptionCategory`))
  (`parent.ReceiveBeginPlay`)
  (bind _output_get (set `self.ConfigBool` (select `bool` (`KismetStringLibrary.EqualEqual_StrStr` _configitemconsumptioncategory "DEFAULT_TRUE") :`false` (`ConfigPropertyBool.Value` (cast `ConfigPropertyBool` (`RuntimeBlueprintFunctionLibrary.Conv_ConfigPropertySectionToConfigProperty` (cast `/SML/ModList/Properties/BP_ConfigPropertySection` (`RuntimeBlueprintFunctionLibrary.Conv_ConfigPropertySectionToConfigProperty` (cast `/SML/ModList/Properties/BP_ConfigPropertySection` (`RuntimeBlueprintFunctionLibrary.Conv_ConfigPropertySectionToConfigProperty` (cast `/SML/ModList/Properties/BP_ConfigPropertySection` (`RuntimeBlueprintFunctionLibrary.Conv_ModConfigurationToConfigProperty` "/ArmorModules/ArmorModules_Configuration.ArmorModules_Configuration_C") :!pure true) "Balance") :!pure true) "ItemConsumption") :!pure true) _configitemconsumptioncategory) :!pure true)) :`true` true)))
  (`/Engine/EditorBlueprintResources/ActorMacros.Switch Has Authority`
    (:`Authority`
      ;[1 1 1] Needs testing
      (`self.ConfigBoolMultiCast` _output_get))))

(event `self.AttachmentPostTick`
  (params (DeltaTime :type "Float (single-precision)"))
  (`parent.AttachmentPostTick` DeltaTime)
  (bind (_has_buffer _consumed) (`self.Check Buffer And Refuel If Needed` (`/ArmorModules/Blueprints/Lib/PSM_Blueprint_Library.Get MAttach Wearing Player` (`self.ParentModule`))))
  (if _consumed
    (if (`FGBlueprintFunctionLibrary.IsLocallyHumanControlled` (`self.GetInstigator`))
      (`self.ModulePlaySound` (`self.RefillSound`) "/ArmorModules/Assets/Audio/RefillEquipSoundConcurrency.RefillEquipSoundConcurrency" 1.0 "NewEnumerator1")))
  ;[1 1 1] Only Consume if we Can  (performance)
  (if _has_buffer
    (`self.Consume Buffer`)))

(event `self.AttachmentInstalled`
  (params (Item :type "InventoryItem Structure"))
  (bind _returnvalue (`FGCharacterPlayer.GetInventory` (`/ArmorModules/Blueprints/Lib/PSM_Blueprint_Library.Get MAttach Wearing Player` (`self.ParentModule`))))
  (`parent.AttachmentInstalled` Item)
  (`/Engine/EditorBlueprintResources/ActorMacros.Switch Has Authority`
    (:`Authority`
      (if (`KismetSystemLibrary.IsValidClass` (`self.LastConsumedItem`))
        (bind _output_get (set `self.Cached Num Posessed Items` (`FGInventoryComponent.GetNumItems` _returnvalue (`self.LastConsumedItem`))))
        (`/ArmorModules/Blueprints/Lib/PSM_Blueprint_Library.Shipping Safe Log` (`KismetStringLibrary.Concat_StrStr` "ItemConsumer Set cached count to " (`KismetStringLibrary.Conv_IntToString` _output_get)) "NewEnumerator3")
        (else
          (bind _output_get_2 (set `self.Cached Num Posessed Items` (`FGInventoryComponent.GetNumItems` _returnvalue (`.ItemClass` (break `ItemAmount` (`|GetArrayItem` (`self.CostToUse`)))))))
          (`/ArmorModules/Blueprints/Lib/PSM_Blueprint_Library.Shipping Safe Log` (`KismetStringLibrary.Concat_StrStr` "ItemConsumer last class was not valid so checking count of first item, got " (`KismetStringLibrary.Conv_IntToString` _output_get_2)) "NewEnumerator1"))))))

(fn `Check Buffer And Refuel If Needed`
  (params (Target :type "FGCharacterPlayer Object Reference"))
  (returns (`Has Buffer` :type Boolean) (Consumed :type Boolean))
  (if (`self.HasAuthority` Target)
    (if (`self.ConfigBool`)
      (if (`/ArmorModules/Blueprints/Lib/PSM_Blueprint_Library.< or Nearly Zero` (`self.CurrentItemStorage%`) (`self.EmptyErrorTolerance`))
        (bind (_consumed _item_class _amount_consumed _num_left) (`/ArmorModules/Blueprints/Lib/PSM_Blueprint_Library.ConsumeItem` Target (`self.CostToUse`)))
        (set `self.Cached Num Posessed Items` _num_left)
        (if _consumed
          (set `self.CurrentItemStorage%` 1.0) ; Refill the internal buffer
          (set `self.LastConsumedItem` _item_class) ; TODO does this really need to be replicated?
          (return true true)
          (else
            (return false false)))
        (else
          (return true false)))
      (else
        ;[1 1 1] If config says we don't need to consume items, always have storage 100% and say the last consumed item was the first one in the list
        (set `self.CurrentItemStorage%` 1.0)
        (set `self.LastConsumedItem` (`.ItemClass` (break `ItemAmount` (`|GetArrayItem` (`self.CostToUse`))))) ; TODO does this really need to be replicated?
        (return true false)))
    (else
      (return true false) ; TODO can client make these assumptions?
    )))

(fn `Check Has One Of These Items`
  (returns (`Found Req'd Item` :type "FGItemDescriptor Class Reference") (`Amount Req'd` :type Integer) (`Inventory Component` :type "FGInventoryComponent Object Reference") (`Has Items?` :type Boolean))
  (bind _returnvalue (`FGCharacterPlayer.GetInventory` (`/ArmorModules/Blueprints/Lib/PSM_Blueprint_Library.Get MAttach Wearing Player` (`self.ParentModule`))))
  (for _array_element (`self.CostToUse`)
    (bind (_itemclass _amount) (break `ItemAmount` _array_element))
    (bind _returnvalue_2 (`FGInventoryComponent.HasItems` _returnvalue _itemclass _amount))
    (if _returnvalue_2
      (return _itemclass _amount _returnvalue _returnvalue_2)))
  (return null 0 _returnvalue false) ; Failed to find
)

(fn `Consume Buffer`
  (locals (`Old Current Item Storage %` :type "Float (double-precision)"))
  (if (`self.ConfigBool`)
    (if (`EquipmentModuleComponent.nProducing` (`self.ParentModule`))
      (bind _modified (`/ArmorModules/Blueprints/Lib/PSM_Blueprint_Library.Item Buffer Consumption Logic` (`self.CurrentItemStorage%`) (`self.EmptyErrorTolerance`) (`self.ChargeLifetime_Seconds`) (`self.DrainIntensityMult`)))
      (if _modified
        (`self.LogCurrentStorageLevel` (`local.Old Current Item Storage %`))))))

(fn `ShouldSave`
  (returns (ReturnValue :type Boolean))
  (return true))

(fn `UserConstructionScript`
  (`parent.UserConstructionScript`))