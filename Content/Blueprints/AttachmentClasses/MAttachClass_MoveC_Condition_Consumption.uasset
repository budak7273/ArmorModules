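; Base power suit attachment class for movement component bonuses conditional on movement mode, meant to be subclassed.
; Enable and disable functions use a flag to apply a signed (+1/-1) modification only once.
; Stat updates clear the flag and re-evaluate the suit state; uninstalling revokes active bonuses.
; The mode switch and modification are unwired templates for derived classes, so this class changes no movement values itself.
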(event `/ArmorModules/Blueprints/AttachmentClasses/MAttachClass_BaseAttachment.OnPowerSuitStatUpdate`
  (params (Type :type Integer))
  (`parent.OnPowerSuitStatUpdate` Type)
  (`/ArmorModules/Blueprints/Lib/PSM_Blueprint_Library.Shipping Safe Log` "Stat update recieved so forcefully saying false" "NewEnumerator5")
  (set `self.CurrentlyApplyingBenefits` false)
  (`self.OnMovementModeChange` "PS_NONE" (`EquipmentModuleComponent.SuitState` (`self.ParentModule`))) ; On install, check their current movement mode\nto see if they should be granted the bonuses
)

(event `/ArmorModules/Blueprints/AttachmentClasses/MAttachClass_BaseAttachment.AttachmentInstalled`
  (params (Item :type "InventoryItem Structure"))
  (`parent.AttachmentInstalled` Item))

(event `/ArmorModules/Blueprints/AttachmentClasses/MAttachClass_BaseAttachment.AttachmentUnInstalled`
  (`parent.AttachmentUnInstalled`)
  (`self.Module Disabled State` "PS_NONE") ; We don't care what the player is doing right now,\nwe must revoke bonuses if they are being given\nbecause the module isn't installed any more
)

(fn `Apply Move C Modification`
  (params (MoveC :type "FGCharacterMovementComponent Object Reference") (`Multiplier for Change to Add to Current Value` :type "Float (double-precision)" :default 1.0) (`Enabling (T) or Disabling(F)` :type Boolean))
  (returns (`New Value` :type "Float (double-precision)"))
  (locals (`MoveC Modifier Created on Derived Blueprint` :type "Float (double-precision)"))
  (return 0.0))

(fn `Module Disabled State`
  (params (`New Move State` :type "EPowerSuitState Enum" :default "PS_NONE"))
  (if (`self.CurrentlyApplyingBenefits`)
    (bind _new_value (`self.Apply Move C Modification` (`EquipmentModuleComponent.MoveC` (`self.ParentModule`)) -1.0))
    (set `self.CurrentlyApplyingBenefits` false)
    (`/ArmorModules/Blueprints/Lib/PSM_Blueprint_Library.Shipping Safe Log` (`KismetStringLibrary.Concat_StrStr` (`KismetSystemLibrary.GetDisplayName` self) " MoveC modification was _disabled_, actual value is now: " (`KismetStringLibrary.Conv_DoubleToString` _new_value)) "NewEnumerator5")
    (else
      (`/ArmorModules/Blueprints/Lib/PSM_Blueprint_Library.Shipping Safe Log` (`KismetStringLibrary.Concat_StrStr` (`KismetSystemLibrary.GetDisplayName` self) " MoveC modification did not need to be removed") "NewEnumerator5"))))

(fn `Module Enabled State`
  (params (`New Move State` :type "EPowerSuitState Enum" :default "PS_NONE"))
  (if (not (`self.CurrentlyApplyingBenefits`))
    (bind _new_value (`self.Apply Move C Modification` (`EquipmentModuleComponent.MoveC` (`self.ParentModule`)) 1.0 true))
    (set `self.CurrentlyApplyingBenefits` true)
    (`/ArmorModules/Blueprints/Lib/PSM_Blueprint_Library.Shipping Safe Log` (`KismetStringLibrary.Concat_StrStr` (`KismetSystemLibrary.GetDisplayName` self) " MoveC modification was  ENABLED,  actual value is now: " (`KismetStringLibrary.Conv_DoubleToString` _new_value)) "NewEnumerator5")
    (else
      (`/ArmorModules/Blueprints/Lib/PSM_Blueprint_Library.Shipping Safe Log` (`KismetStringLibrary.Concat_StrStr` (`KismetSystemLibrary.GetDisplayName` self) " MoveC modification did not need to be added") "NewEnumerator5"))))

(fn `OnMovementModeChange`
  (params (`Previous Movement Mode` :type "EPowerSuitState Enum" :default "PS_NONE") (`New Movement Mode` :type "EPowerSuitState Enum" :default "PS_NONE"))
  (`parent.OnMovementModeChange` `Previous Movement Mode` `New Movement Mode`))

(fn `UserConstructionScript`
  (`parent.UserConstructionScript`))