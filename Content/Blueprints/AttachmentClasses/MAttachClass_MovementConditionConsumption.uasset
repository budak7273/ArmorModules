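; Suit module attachment that sets power and fuel drain by the suit's movement state and plays state transition sounds.
; Per-state cost maps, with fallbacks for unlisted states, drive both drains; fuel adds to the parent's value.
; Listed costs scale while the boost key is held (missing toggle sprint), and power also when fuel is empty.
; Tick detects state changes, playing exact or NONE-wildcard sound matches for the local player only.
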(event `self.AttachmentTick`
  (params (DeltaTime :type "Float (single-precision)"))
  (bind __lastmovementstate (`self._LastMovementState`))
  (bind _suitstate (`EquipmentModuleComponent.SuitState` (`self.ParentModule`)))
  (`parent.AttachmentTick` DeltaTime)
  (if (not (== __lastmovementstate _suitstate))
    (`self.OnMovementModeChange` __lastmovementstate _suitstate))
  (set `self._LastMovementState` _suitstate))

(fn `ArmorModules Get Delta Fuel Consumption`
  (params (`Delta Time` :type "Float (double-precision)") (`PreCalc'd Fuel Consumption` :type "Float (double-precision)"))
  (returns (DeltaTime_ :type "Float (double-precision)") (`Fuel Consumption` :type "Float (double-precision)"))
  (bind _parentmodule (`self.ParentModule`))
  (bind (_value _returnvalue) (`BlueprintMapLibrary.Map_Find` (`self.FuelCostMW`) (`EquipmentModuleComponent.SuitState` _parentmodule)))
  (bind (_deltatime_ _fuel_consumption) (`parent.ArmorModules Get Delta Fuel Consumption` `Delta Time` `PreCalc'd Fuel Consumption`))
  (if _returnvalue
    (return _deltatime_ (+ (* (select `bool` (`EMC_StateModule.HKey_Accel` (`EquipmentModuleComponent.StateModule` _parentmodule)) :`false` 1.0 :`true` (`self.SprintingFuelCostMult`)) _value) _fuel_consumption))
    (else
      (return _deltatime_ (+ _fuel_consumption (`self.FuelCostForUnspecifiedStatesMW`))))))

(fn `GetDeltaPowerConsumption`
  (params (DeltaTime :type "Float (double-precision)"))
  (returns (ReturnValue :type "Float (double-precision)"))
  (bind _parentmodule (`self.ParentModule`))
  (bind (_value _returnvalue) (`BlueprintMapLibrary.Map_Find` (`self.PowerCostMW`) (`EquipmentModuleComponent.SuitState` _parentmodule)))
  (if _returnvalue
    (return (* (`KismetMathLibrary.SelectFloat` 1.0 (`self.OutOfFuelPowerCostMult`) (> (`EquipmentModuleComponent.nFuelAmount` _parentmodule) 0.0)) (`KismetMathLibrary.SelectFloat` (`self.SprintingPowerCostMult`) 1.0 (`EMC_StateModule.HKey_Accel` (`EquipmentModuleComponent.StateModule` _parentmodule))) _value))
    (else
      (return (`self.PowerCostForUnspecifiedStatesMW`)))))

(fn `OnMovementModeChange`
  (params (`Previous Movement Mode` :type "EPowerSuitState Enum" :default "PS_NONE") (`New Movement Mode` :type "EPowerSuitState Enum" :default "PS_NONE"))
  (locals (SoundToPlay :type "SoundBase Object Reference"))
  (bind _movestate_transition_sounds (`self.MoveState Transition Sounds`))
  (bind (_value _returnvalue) (`BlueprintMapLibrary.Map_Find` _movestate_transition_sounds (make `/ArmorModules/Blueprints/Lib/SuitStateTransition` `Previous Movement Mode`)))
  (bind (_value_2 _returnvalue_2) (`BlueprintMapLibrary.Map_Find` _movestate_transition_sounds (make `/ArmorModules/Blueprints/Lib/SuitStateTransition` `Previous Movement Mode` `New Movement Mode`)))
  (bind (_value_3 _returnvalue_3) (`BlueprintMapLibrary.Map_Find` _movestate_transition_sounds (make `/ArmorModules/Blueprints/Lib/SuitStateTransition` "PS_NONE" `New Movement Mode`)))
  (`/ArmorModules/Blueprints/Lib/PSM_Blueprint_Library.Shipping Safe Log` (`KismetStringLibrary.Concat_StrStr` "New movement mode is: " (`|GetEnumeratorNameAsString` `New Movement Mode`) " Boost Keydown is: " (`KismetStringLibrary.Conv_BoolToString` (`EMC_StateModule.HKey_Accel` (`EquipmentModuleComponent.StateModule` (`self.ParentModule`))))) "NewEnumerator3")
  (if (`FGBlueprintFunctionLibrary.IsLocallyHumanControlled` (`self.GetInstigator`))
    (if (> (`BlueprintMapLibrary.Map_Length` (`self.MoveState Transition Sounds`)) 0)
      ;[1 1 1] Try to find the most relevant sound to play for the transition
      (set `local.SoundToPlay` null) ; Reset
      (if _returnvalue_2
        (set `local.SoundToPlay` _value_2)
        (`self.ModulePlaySound` (`local.SoundToPlay`) :!label _label) ; TODO pick concurrency and category
        (return)
        (elif _returnvalue
          (set `local.SoundToPlay` _value)
          (goto _label)
          (elif _returnvalue_3
            (set `local.SoundToPlay` _value_3)
            (goto _label))))
      (else
        (return)))
    (else
      (return))))

(fn `UserConstructionScript`
  (`parent.UserConstructionScript`))