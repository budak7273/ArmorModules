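; Power suit attachment that handles Rob refuel logic, keeping an item-based fuel buffer for the parent module.
; On install it builds its use cost from one of each fuel the fuel module allows and binds to suit stat updates, which recompute transfer rates.
; Each tick RobRefuelOnTickLogic updates the buffer; post-tick logs its energy in MJ, scaled by suit fuel efficiency.
; Several tank and buffer helpers are unused.
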(event `/ArmorModules/Blueprints/AttachmentClasses/MAttachClass_BaseAttachment.AttachmentInstalled`
  (params (Item :type "InventoryItem Structure"))
  (`parent.AttachmentInstalled` Item)
  (`KismetArrayLibrary.Array_Clear` (`self._BuildItemAmount`))
  (for _array_element (`EMC_FuelModule.nAllowedFuels` (`EquipmentModuleComponent.FuelModule` (`self.ParentModule`)))
    (`KismetArrayLibrary.Array_Add` (`self._BuildItemAmount`) (make `ItemAmount` _array_element 1)))
  (set `self.CostToUse` (`self._BuildItemAmount`))
  (`/ArmorModules/Blueprints/Lib/PSM_Blueprint_Library.Shipping Safe Log` "Done building new cost to use")
  (add `PowerSuit.OnPowerSuitStatUpdate` (`EquipmentModuleComponent.EquipmentParent` (`self.ParentModule`)) (delegate `OnPowerSuitStatUpdate_Event_0`)))

(event `OnPowerSuitStatUpdate_Event_0`
  (params (Type :type Integer))
  (bind (_percentoftankper1second _mjper1second) (break `/ArmorModules/Blueprints/Lib/FuelTransferSpeedSpecification` (`self.Fuel Transfer Speed`)))
  (bind (_percentoftankper1second_2 _mjper1second_2) (break `/ArmorModules/Blueprints/Lib/FuelTransferSpeedSpecification` (`/ArmorModules/Blueprints/Lib/PSM_Blueprint_Library.Get Effective Fuel Transfer Speed of Suit` (`self.ParentModule`))))
  (set `self.PercentOfTankPerSec` (+ _percentoftankper1second _percentoftankper1second_2))
  (set `self.MJ PerSec` (+ _mjper1second _mjper1second_2)))

(event `self.AttachmentPostTick`
  (params (DeltaTime :type "Float (single-precision)"))
  (`parent.AttachmentPostTick` DeltaTime)
  (`/ArmorModules/Blueprints/Lib/PSM_Blueprint_Library.Shipping Safe Log` (`KismetStringLibrary.Concat_StrStr` "Energy equivalent of buffer is " (`KismetStringLibrary.Conv_DoubleToString` (`self.Current Storage Energy Equivalent MJ`))) "NewEnumerator5"))

(event `self.AttachmentTick`
  (params (DeltaTime :type "Float (single-precision)"))
  (`parent.AttachmentTick` DeltaTime)
  (bind _new_currentitemstorage_ (`/ArmorModules/Blueprints/Lib/PSM_Blueprint_Library.RobRefuel On Tick Logic` (`self.ParentModule`) (`self.CurrentItemStorage%`) 0.0001 (`self.LastConsumedItem`)))
  (set `self.CurrentItemStorage%` _new_currentitemstorage_))

(fn `Current Storage Energy Equivalent MJ`
  (returns (`Energy MJ` :type "Float (double-precision)") (`Energy MJ Before Suit Fuel Efficiency` :type "Float (double-precision)"))
  (bind _mj (`self.Fuel% to MJ ` (`self.CurrentItemStorage%`) (`FGItemDescriptor.GetEnergyValue` (`self.LastConsumedItem`))))
  (return (* _mj (`/ArmorModules/Blueprints/Lib/PSM_Blueprint_Library.Get Suit 1-based Fuel Efficiency Safe` (`self.ParentModule`))) _mj))

(fn `Fuel% to MJ `
  (params (`Buffer Fill %` :type "Float (double-precision)") (`Tank Size MJ` :type "Float (double-precision)"))
  (returns (MJ :type "Float (double-precision)"))
  (return (* `Buffer Fill %` `Tank Size MJ`)))

(fn `UserConstructionScript`
  (`parent.UserConstructionScript`))