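; Suit shield attachment that handles shield damage, audio feedback and power draw.
; On locally human-controlled owners it registers a health-component adjust-damage listener, passing damage through the parent module's CalculateDamage, returning the remainder and playing hit or break sounds.
; Tick compares shield and cooldown state against the last tick to play recharge-start and full sounds.
; Power consumption charges a maintain cost while shielded and a higher cost while recharging.
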(event `self.AttachmentTick`
  (params (DeltaTime :type "Float (single-precision)"))
  (bind _parentmodule (`self.ParentModule`))
  (bind _ncurrentshield (`EquipmentModuleComponent.nCurrentShield` _parentmodule))
  (bind _nshieldregencooldown (`EquipmentModuleComponent.nShieldRegenCooldown` (`self.ParentModule`)))
  (bind _returnvalue (`EMC_ShieldModule.GetMaxShield` (`EquipmentModuleComponent.ShieldModule` _parentmodule)))
  (`parent.AttachmentTick` DeltaTime)
  ;[1 1 1] Begin Recharging sound
  (if (and (not _nshieldregencooldown) (`self._WasOnCooldownLastTick`))
    (`self.ModulePlaySound` (`self.Shield Start Recharge Sound`) "/ArmorModules/Assets/Audio/ShieldSoundConcurrency.ShieldSoundConcurrency" 1.0 1.0 "NewEnumerator3"))
  (set `self._WasOnCooldownLastTick` _nshieldregencooldown)
  ;[1 1 1] Shield Done Recharging sound
  (if (and (>= _ncurrentshield _returnvalue) (< (`self._ShieldLastTick`) _returnvalue))
    (`self.ModulePlaySound` (`self.Shield Full Sound`) "/ArmorModules/Assets/Audio/ShieldSoundConcurrency.ShieldSoundConcurrency" 1.0 1.0 "NewEnumerator3"))
  (set `self._ShieldLastTick` _ncurrentshield))

(event `self.AttachmentUnInstalled`
  ;[1 1 1] Damage listener attach/detach
  (`parent.AttachmentUnInstalled`)
  (if (`FGBlueprintFunctionLibrary.IsLocallyHumanControlled` (`self.GetInstigator`))
    (`FGHealthComponent.RemoveAdjustDamageListener` (`FGCharacterBase.GetHealthComponent` (`/ArmorModules/Blueprints/Lib/PSM_Blueprint_Library.Get MAttach Wearing Player` (`self.ParentModule`))) (`|CreateDelegate` :!event `On Take Damage Handler`))
    (`/ArmorModules/Blueprints/Lib/PSM_Blueprint_Library.Shipping Safe Log` "Removed AdjustDamageListener" "NewEnumerator5")))

(event `self.AttachmentInstalled`
  (params (Item :type "InventoryItem Structure"))
  ;[1 1 1] Damage listener attach/detach
  (`parent.AttachmentInstalled` Item)
  (if (`FGBlueprintFunctionLibrary.IsLocallyHumanControlled` (`self.GetInstigator`))
    (`FGHealthComponent.AddAdjustDamageListener` (`FGCharacterBase.GetHealthComponent` (`/ArmorModules/Blueprints/Lib/PSM_Blueprint_Library.Get MAttach Wearing Player` (`self.ParentModule`))) (`|CreateDelegate` :!event `On Take Damage Handler`))
    (`/ArmorModules/Blueprints/Lib/PSM_Blueprint_Library.Shipping Safe Log` "Attached AdjustDamageListener" "NewEnumerator5")))

(event `On Parent Shield Damage Take`
  (params (ShieldDamage :type "Float (double-precision)") (Date :type "DateTime Structure") (empty :type Boolean) (Impact :type "HitResult Structure"))
  ;[1 1 1] TODO remove me, does not seem to work and was replaced by health listener
)

(fn `GetDeltaPowerConsumption`
  (params (DeltaTime :type "Float (double-precision)"))
  (returns (ReturnValue :type "Float (double-precision)"))
  (bind _parentmodule (`self.ParentModule`))
  (bind _ncurrentshield (`EquipmentModuleComponent.nCurrentShield` _parentmodule))
  (return (+ (select `bool` (> _ncurrentshield 0.0) :`false` 0.0 :`true` (`self.ShieldMaintainPowerCostMW`)) (select `bool` (and (< _ncurrentshield (`EMC_ShieldModule.GetMaxShield` (`EquipmentModuleComponent.ShieldModule` _parentmodule))) (not (`EquipmentModuleComponent.nShieldRegenCooldown` _parentmodule))) :`false` 0.0 :`true` (- (`self.ShieldRechargingPowerCostMW`) (`self.ShieldMaintainPowerCostMW`))))))

(fn `On Take Damage Handler`
  (params (damagedActor :type "Actor Object Reference") (damageAmount :type "Float (double-precision)") (damageType :type "DamageType Object Reference") (instigatedBy :type "Controller Object Reference") (damageCauser :type "Actor Object Reference"))
  (returns (ReturnValue :type "Float (double-precision)"))
  (bind (_soundbase _pitch_mult) (`self.Random shield sound and pitch`))
  (bind (_asfgdamage_type _bsuccess) (cast `FGDamageType` damageType :!pure true))
  (if (> damageAmount 0.0)
    (set `self.ShieldBeforeCalculateDamage` (`EquipmentModuleComponent.nCurrentShield` (`self.ParentModule`)))
    (if true
      (bind _returnvalue (`EquipmentModuleComponent.CalculateDamage` :`self` (`self.ParentModule`) :`DmgIn` damageAmount :`Type` (select `bool` _bsuccess :`false` 1 :`true` (`/PowerSuit/Util/Lib_GetDamageTypeMask.GetDamageTypeMask` _asfgdamage_type)) :`BpType` (select `bool` _bsuccess :`false` "/Script/FactoryGame.FGDamageType" :`true` (`GameplayStatics.GetObjectClass` _asfgdamage_type)))) ; Factor in damage resistances, then apply the damage to the shield\n\nTODO ensure it isn't taking double damage\n(does the suit also end up calling this?)\nDoesn't seem to be doubling it based on testing fall damage
      ;[1 1 1] Decide which sound to play (shield hit, break, or none)
      (`/ArmorModules/Blueprints/Lib/PSM_Blueprint_Library.Shipping Safe Log` (`KismetStringLibrary.Concat_StrStr` "Health damage after shield calculate was " (`KismetStringLibrary.Conv_DoubleToString` _returnvalue)) "NewEnumerator5")
      (if (> (`self.ShieldBeforeCalculateDamage`) 0.0)
        (if (< (`EquipmentModuleComponent.nCurrentShield` (`self.ParentModule`)) (`self.ShieldBeforeCalculateDamage`))
          (if (<= (`EquipmentModuleComponent.nCurrentShield` (`self.ParentModule`)) 0.0)
            (`/ArmorModules/Blueprints/Lib/PSM_Blueprint_Library.Shipping Safe Log` "Shield break" "NewEnumerator3")
            (`self.ModulePlaySound` (`self.Shield Break Sound`) "/ArmorModules/Assets/Audio/ShieldSoundConcurrency.ShieldSoundConcurrency" 1.0 1.0 "NewEnumerator3")
            (else
              (`/ArmorModules/Blueprints/Lib/PSM_Blueprint_Library.Shipping Safe Log` "Played sound" "NewEnumerator5")
              (`self.ModulePlaySound` _soundbase "/ArmorModules/Assets/Audio/ShieldSoundConcurrency.ShieldSoundConcurrency" _pitch_mult 1.0 "NewEnumerator3")))
          (else
            (`/ArmorModules/Blueprints/Lib/PSM_Blueprint_Library.Shipping Safe Log` "Shield was down OR not a blocked damage type" "NewEnumerator5" :!label _label)))
        (else
          (goto _label)))
      (return _returnvalue) ; Any excess damage\nflows through to be\ndealt to the player
      (else
        (`/ArmorModules/Blueprints/Lib/PSM_Blueprint_Library.Shipping Safe Log` "Suit does not have shield flag for this \nkind of damage, ")
        (return damageAmount)))
    (else
      (`/ArmorModules/Blueprints/Lib/PSM_Blueprint_Library.Shipping Safe Log` "Zero damage was dealt, so no need to continue shield logic" "NewEnumerator5"))))

(fn `Random shield sound and pitch`
  (returns (SoundBase :type "SoundBase Object Reference") (`Pitch Mult` :type "Float (double-precision)"))
  (return (select `int` (`KismetMathLibrary.RandomInteger` 2) :`0` "/PowerSuit/Assets/GitIgnoredAssets/AudioSrc/Shield/shield_hit_2.shield_hit_2" :`1` "/PowerSuit/Assets/GitIgnoredAssets/AudioSrc/Shield/shield_hit_3.shield_hit_3" :!type "SoundBase Object Reference") (`KismetMathLibrary.RandomFloatInRange` 0.9 1.1)))

(fn `UserConstructionScript`
  (`parent.UserConstructionScript`))