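; Attachment class Blueprint that holds a configurable slider value.
; UpdateSliderValue stores the new value, logs the change through ShippingSafeLog with shipping output disabled, and returns the previous value.
; The construction script only calls its parent, and the file shows no further effect of the value.
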(fn `Update Slider Value`
  (params (`New Value` :type "Float (double-precision)"))
  (returns (`Old Value` :type "Float (double-precision)"))
  (locals (`Old Val` :type "Float (double-precision)" :default 0.0))
  (set `local.Old Val` (`self.Slider Value`))
  (bind _output_get (set `self.Slider Value` `New Value`))
  (`/ArmorModules/Blueprints/Lib/PSM_Blueprint_Library.Shipping Safe Log` (`KismetStringLibrary.Concat_StrStr` "Slider value changed from " (`KismetStringLibrary.Conv_DoubleToString` (`local.Old Val`)) " to " (`KismetStringLibrary.Conv_DoubleToString` _output_get)) "NewEnumerator3")
  (return (`local.Old Val`)))

(fn `UserConstructionScript`
  (`parent.UserConstructionScript`))