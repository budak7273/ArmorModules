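; Config subsystem for the Armor Modules mod that loads its debugging settings from the mod configuration.
; On BeginPlay it binds to changes in the Debugging section and runs the same handler for the initial load.
; The handler caches the logging flags and suit HUD debug mode, then logs them, even in shipping builds.
; It is not saved, and an unwired sub-mod loaded check remains in the graph.
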(event `On PSM Debugging Settings Changed`
  (bind _asbp_config_property_section (cast `/SML/ModList/Properties/BP_ConfigPropertySection` (`RuntimeBlueprintFunctionLibrary.Conv_ConfigPropertySectionToConfigProperty` (cast `/SML/ModList/Properties/BP_ConfigPropertySection` (`RuntimeBlueprintFunctionLibrary.Conv_ModConfigurationToConfigProperty` "/ArmorModules/ArmorModules_Configuration.ArmorModules_Configuration_C") :!pure true) "Debugging") :!pure true))
  (bind _output_get (set `self.EnableLogs` (`ConfigPropertyBool.Value` (cast `ConfigPropertyBool` (`RuntimeBlueprintFunctionLibrary.Conv_ConfigPropertySectionToConfigProperty` _asbp_config_property_section "EnableLogs") :!pure true))))
  (bind _output_get_2 (set `self.EvenLogDisabled` (`ConfigPropertyBool.Value` (cast `ConfigPropertyBool` (`RuntimeBlueprintFunctionLibrary.Conv_ConfigPropertySectionToConfigProperty` _asbp_config_property_section "EvenLogDisabled") :!pure true))))
  (bind _output_get_3 (set `self.SuitHudDebugMode` (`RuntimeBlueprintFunctionLibrary.Conv_ConfigPropertyToInteger` (`RuntimeBlueprintFunctionLibrary.Conv_ConfigPropertySectionToConfigProperty` _asbp_config_property_section "HudDebugMode"))))
  (`/ArmorModules/Blueprints/Lib/PSM_Blueprint_Library.Shipping Safe Log` (`KismetStringLibrary.Concat_StrStr` "Loaded logging settings: Enabled?: " (`KismetStringLibrary.Conv_BoolToString` _output_get) "   Everything?: " (`KismetStringLibrary.Conv_BoolToString` _output_get_2) " HUD Debug Mode: " (`KismetStringLibrary.Conv_IntToString` _output_get_3)) "NewEnumerator3" true))

(event `self.ReceiveBeginPlay`
  (add `ConfigProperty.OnPropertyValueChanged` (`RuntimeBlueprintFunctionLibrary.Conv_ConfigPropertySectionToConfigProperty` (cast `/SML/ModList/Properties/BP_ConfigPropertySection` (`RuntimeBlueprintFunctionLibrary.Conv_ModConfigurationToConfigProperty` "/ArmorModules/ArmorModules_Configuration.ArmorModules_Configuration_C") :!pure true) "Debugging") (delegate `On PSM Debugging Settings Changed`))
  (`self.On PSM Debugging Settings Changed`))

(fn `GatherDependencies`
  (returns (out_dependentObjects :type "Array of Object Object Reference"))
  (return))

(fn `NeedTransform`
  (returns (ReturnValue :type Boolean))
  (return false))

(fn `ShouldSave`
  (returns (ReturnValue :type Boolean))
  (return false))

(fn `UserConstructionScript`)