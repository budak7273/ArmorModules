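; Mod subsystem that keeps the registry of sluggable items for ArmorModules.
; BeginPlay registers the default items, and register and remove functions edit the collection, log the outcome and report success.
; The getter returns the collection or, if it is empty, requests the server's copy and flags a retry.
; An author note says that RPC path likely never runs, as the subsystem spawns on both sides without replication.
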(event `self.ReceiveBeginPlay`
  (`self.Register Default Items`))

(event `Request Authority Send Sluggable Items`
  ;[1 1 1] When I marked this subsystem as to be replicated, I don't think any of this is ever really called.
  ;
  ; I saw error messages for "LogNet: Warning: UNetDriver::ProcessRemoteFunction: No owning connection for actor ArmorModules_SluggableItemsSubsystem_C_2147480599. Function Request Authority Send Sluggable Items will not be processed."
  ;
  ; I instead marked as Spawn on Both, Never Replicate, to let each side handle it, because there is not really a case where server decides to add something that client would not know about (yet)
  (`/ArmorModules/Blueprints/Lib/PSM_Blueprint_Library.Shipping Safe Log` "Authority sending sluggable Items to clients")
  (`self.Client Received Sluggable Items` (`self.Sluggable Items`)))

(event `Client Received Sluggable Items`
  (params (`Sluggable Items from Server` :type "Set of /ArmorModules/Blueprints/Lib/SlugItemFalloff Structure"))
  ;[1 1 1] When I marked this subsystem as to be replicated, I don't think any of this is ever really called.
  ;
  ; I saw error messages for "LogNet: Warning: UNetDriver::ProcessRemoteFunction: No owning connection for actor ArmorModules_SluggableItemsSubsystem_C_2147480599. Function Request Authority Send Sluggable Items will not be processed."
  ;
  ; I instead marked as Spawn on Both, Never Replicate, to let each side handle it, because there is not really a case where server decides to add something that client would not know about (yet)
  (`/ArmorModules/Blueprints/Lib/PSM_Blueprint_Library.Shipping Safe Log` (`KismetStringLibrary.Concat_StrStr` "Client got " (`KismetStringLibrary.Conv_IntToString` (`BlueprintSetLibrary.Set_Length` `Sluggable Items from Server`)) " sluggable items from server: "))
  (`|ExecutionSequence`
    (:`then_0`
      (bind _result (`BlueprintSetLibrary.Set_ToArray` `Sluggable Items from Server`))
      (for _array_element _result
        (`/ArmorModules/Blueprints/Lib/PSM_Blueprint_Library.Shipping Safe Log` (`KismetTextLibrary.Conv_TextToString` (`FGItemDescriptor.GetItemName` (`.Item_2_00C9F7734A6FD120E492BFB4C503E78B` (break `/ArmorModules/Blueprints/Lib/SlugItemFalloff` _array_element)))) "NewEnumerator3")))
    (:`then_1`
      (set `self.Sluggable Items` `Sluggable Items from Server`))))

(fn `Get Sluggable Items`
  (returns (Structs :type "Set of /ArmorModules/Blueprints/Lib/SlugItemFalloff Structure") (NeedsRetryAfterRep :type Boolean))
  (if (> (`BlueprintSetLibrary.Set_Length` (`self.Sluggable Items`)) 0)
    (return (`self.Sluggable Items`) false)
    (else
      (`/ArmorModules/Blueprints/Lib/PSM_Blueprint_Library.Shipping Safe Log` "My sluggable items copy is 0 so requesting new from server" "NewEnumerator1")
      (`self.Request Authority Send Sluggable Items`)
      (return _ true))))

(fn `Register Default Items`
  (`/ArmorModules/Blueprints/Lib/PSM_Blueprint_Library.Shipping Safe Log` "Init default sluggable items" "NewEnumerator3")
  (for _array_element (`self.DefaultSluggableItems`)
    (`self.Register Sluggable Item` _array_element)))

(fn `Register Sluggable Item`
  (params (Struct :type "/ArmorModules/Blueprints/Lib/SlugItemFalloff Structure"))
  (returns (Success :type Boolean))
  (locals (AlreadyHad :type Boolean :default false))
  (bind _sluggable_items (`self.Sluggable Items`))
  (bind _output_get (set `local.AlreadyHad` (`BlueprintSetLibrary.Set_Contains` _sluggable_items Struct)))
  (if (not _output_get)
    (`BlueprintSetLibrary.Set_Add` _sluggable_items Struct))
  (`/ArmorModules/Blueprints/Lib/PSM_Blueprint_Library.Shipping Safe Log` (`KismetStringLibrary.Concat_StrStr` "Registering sluggable item: " (`KismetSystemLibrary.GetClassDisplayName` (`.Item_2_00C9F7734A6FD120E492BFB4C503E78B` (break `/ArmorModules/Blueprints/Lib/SlugItemFalloff` Struct))) " Success?: " (`KismetStringLibrary.Conv_BoolToString` (not (`local.AlreadyHad`)))) "NewEnumerator3")
  (return (not (`local.AlreadyHad`))))

(fn `Remove Sluggable Item`
  (params (Struct :type "/ArmorModules/Blueprints/Lib/SlugItemFalloff Structure"))
  (returns (Success :type Boolean))
  (bind _returnvalue (`BlueprintSetLibrary.Set_Remove` (`self.Sluggable Items`) Struct))
  (`/ArmorModules/Blueprints/Lib/PSM_Blueprint_Library.Shipping Safe Log` (`KismetStringLibrary.Concat_StrStr` "Unregistered sluggable item: " (`KismetSystemLibrary.GetClassDisplayName` (`.Item_2_00C9F7734A6FD120E492BFB4C503E78B` (break `/ArmorModules/Blueprints/Lib/SlugItemFalloff` Struct))) " Success?: " (`KismetStringLibrary.Conv_BoolToString` _returnvalue)) "NewEnumerator3")
  (return _returnvalue))

(fn `UserConstructionScript`)