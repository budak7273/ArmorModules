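; Tooltip spawner that adds a Somersloop info widget to item tooltips in the ArmorModules mod.
; CreateDescriptionWidget creates the widget only when the ModuleTooltips setting in the mod configuration is enabled and the stack's item class is in ItemsToDisplayOn.
; GetItemDescription returns an empty string, so the widget is the only content it contributes.
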(fn `CreateDescriptionWidget`
  (params (OwningPlayer :type "PlayerController Object Reference") (InventoryStack :type "InventoryStack Structure (by ref)"))
  (returns (ReturnValue :type "Widget Object Reference"))
  (if (`ConfigPropertyBool.Value` (cast `/SML/ModList/Properties/BP_ConfigPropertyBool` (`RuntimeBlueprintFunctionLibrary.Conv_ConfigPropertySectionToConfigProperty` (cast `/SML/ModList/Properties/BP_ConfigPropertySection` (`RuntimeBlueprintFunctionLibrary.Conv_ModConfigurationToConfigProperty` "/ArmorModules/ArmorModules_Configuration.ArmorModules_Configuration_C") :!pure true) "ModuleTooltips") :!pure true))
    (if (`BlueprintSetLibrary.Set_Contains` (`self.ItemsToDisplayOn`) (`FGInventoryLibrary.BreakInventoryItem` (`.out_item` (`FGInventoryLibrary.BreakInventoryStack` InventoryStack))))
      (bind _returnvalue (`|CreateWidget` "/ArmorModules/Blueprints/ToolTips/Widget_SomersloopInfo.Widget_SomersloopInfo_C" OwningPlayer))
      (return _returnvalue)
      (else
        (return null)))
    (else
      (return null))))

(fn `GetItemDescription`
  (params (OwningPlayer :type "PlayerController Object Reference") (InventoryStack :type "InventoryStack Structure (by ref)"))
  (returns (ReturnValue :type Text))
  (return ""))

(fn `UserConstructionScript`)