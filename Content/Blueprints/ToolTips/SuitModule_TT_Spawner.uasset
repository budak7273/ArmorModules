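; Tooltip provider for the Armor Modules mod that supplies a rich description widget for suit modules and modular suits.
; CreateDescriptionWidget first checks the ModuleTooltips config option, then accepts items whose class is an equipment module descriptor or whose state is an armor modules suit.
; Matching items get an initialized Widget_RichModuleTooltip built from the inventory stack's item; all others get no widget, and the text description is always empty.
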(fn `CreateDescriptionWidget`
  (params (OwningPlayer :type "PlayerController Object Reference") (InventoryStack :type "InventoryStack Structure (by ref)"))
  (returns (ReturnValue :type "Widget Object Reference"))
  (bind (_out_numitems _out_item) (`FGInventoryLibrary.BreakInventoryStack` InventoryStack))
  (bind (_out_itemclass _out_itemstate) (`FGInventoryLibrary.BreakInventoryItem` _out_item))
  (if (`ConfigPropertyBool.Value` (cast `/SML/ModList/Properties/BP_ConfigPropertyBool` (`RuntimeBlueprintFunctionLibrary.Conv_ConfigPropertySectionToConfigProperty` (cast `/SML/ModList/Properties/BP_ConfigPropertySection` (`RuntimeBlueprintFunctionLibrary.Conv_ModConfigurationToConfigProperty` "/ArmorModules/ArmorModules_Configuration.ArmorModules_Configuration_C") :!pure true) "ModuleTooltips") :!pure true))
    (castclass `EquipmentModuleDescriptor` _out_itemclass ; Is it an equip descriptor?
      (:`then`
        _)
      (:`CastFailed`
        (`/Engine/EditorBlueprintResources/StandardMacros.IsValid` _out_itemstate
          (:`Is Valid`
            (cast `/ArmorModules/Blueprints/EquipClass_ArmorModulesSuit` _out_itemstate ; Is it a suit (according to state)
              (:`then`
                _)
              (:`CastFailed`
                (return null))))
          (:`Is Not Valid`
            (return null)))))
    (bind _returnvalue (`|CreateWidget` "/ArmorModules/Blueprints/ToolTips/Widget_RichModuleTooltip.Widget_RichModuleTooltip_C" OwningPlayer _out_item))
    (set `/ArmorModules/Blueprints/ToolTips/Widget_RichModuleTooltip.Item` _out_item _returnvalue)
    (set `/ArmorModules/Blueprints/ToolTips/Widget_RichModuleTooltip.Class` _out_itemclass _returnvalue)
    (`/ArmorModules/Blueprints/ToolTips/Widget_RichModuleTooltip.Init` _returnvalue)
    (return _returnvalue)
    (else
      (return null))))

(fn `GetItemDescription`
  (params (OwningPlayer :type "PlayerController Object Reference") (InventoryStack :type "InventoryStack Structure (by ref)"))
  (returns (ReturnValue :type Text))
  (return ""))

(fn `UserConstructionScript`)