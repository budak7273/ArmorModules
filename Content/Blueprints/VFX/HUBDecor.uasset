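; Decor actor for the HUB that manages a synced wormhole, its teleport effect and a random easter egg.
; Wormhole visibility follows whether its schematic is purchased, refreshed at BeginPlay and on each purchase.
; PlayTeleportAnimation fires a dispatcher whose handler spawns a TeleportLeftBehind actor at the wormhole's transform.
; Hub-destruction handling here is obsolete and unwired, as the game world module now handles it.
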(event `TeleportAnim_Event`
  (`/ArmorModules/Blueprints/Lib/PSM_Blueprint_Library.Shipping Safe Log` "HUBDecor running TeleportAnim" "NewEnumerator3")
  (`|SpawnActorFromClass` "/ArmorModules/Blueprints/VFX/TeleportLeftBehind.TeleportLeftBehind_C" (`SceneComponent.K2_GetComponentToWorld` (`self.SyncedWormhole`)) "AlwaysSpawn" "OverrideRootScale" null 5.0 (`KismetMathLibrary.MakeVector` 3.165 3.165 3.165) null))

(event `self.ReceiveBeginPlay`
  (`|ExecutionSequence`
    (:`then_0`
      (`SceneComponent.SetVisibility` (`self.EasterEgg_1`) (`/ArmorModules/Blueprints/Lib/PSM_Blueprint_Library.Try Easter Egg Occurance` 100) true))
    (:`then_1`
      (add `self.TeleportAnim` (delegate `TeleportAnim_Event`))
      (add `FGSchematicManager.PurchasedSchematicDelegate` (`FGSchematicManager.Get` self) (delegate `OnSchemPurchased`))
      (`self.Update Visibility`))))

(event `OnSchemPurchased`
  (params (purchasedSchematic :type "FGSchematic Class Reference"))
  (`self.Update Visibility`))

(event `HubDestroyed` :!signature `self.OnDestroyed`
  (params (DestroyedActor :type "Actor Object Reference"))
  ;[1 1 1] Should no longer be needed
  (`/ArmorModules/Blueprints/Lib/PSM_Blueprint_Library.Shipping Safe Log` "Decor's Hub destroyed event"))

(event `self.ReceiveTick`
  (params (DeltaSeconds :type "Float (single-precision)")))

(fn `Play Teleport Animation`
  (`self.TeleportAnim`))

(fn `Update Visibility`
  (`SceneComponent.SetVisibility` (`self.SyncedWormhole`) (`FGSchematicManager.IsSchematicPurchased` (`FGSchematicManager.Get` self) "/ArmorModules/Schematics/TreeNodes/Node_Craft_FreshSyncedWormhole.Node_Craft_FreshSyncedWormhole_C") false))

(fn `UserConstructionScript`)