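; TeleportLeftBehind is a short-lived VFX actor, apparently the remnant left behind by a teleport, that shrinks away while playing a sound.
; BeginPlay starts the audio, schedules its stop, then destroys the actor after the animation duration, with debug logging along the way.
; Tick lerps the current scale toward zero by elapsed-time fraction, compounding each frame into an accelerating, frame-rate-dependent shrink.
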(event `self.ReceiveDestroyed`
  (`AudioComponent.Stop` (`self.Audio`)))

(event `self.ReceiveBeginPlay`
  (bind _animationdurationseconds (`self.AnimationDurationSeconds`))
  (bind _audio (`self.Audio`))
  (`/ArmorModules/Blueprints/Lib/PSM_Blueprint_Library.Shipping Safe Log` "LeftBehind spawned" "NewEnumerator3")
  (`AudioComponent.Play` _audio 0.0)
  (`AudioComponent.StopDelayed` _audio _animationdurationseconds)
  (`KismetSystemLibrary.Delay` _animationdurationseconds)
  (`/ArmorModules/Blueprints/Lib/PSM_Blueprint_Library.Shipping Safe Log` "LeftBehind destroy" "NewEnumerator3")
  (`self.K2_DestroyActor`))

(event `self.ReceiveTick`
  (params (DeltaSeconds :type "Float (single-precision)"))
  (bind _currentscale (`self.CurrentScale`))
  (bind _output_get (set `self.CurrentLifetimeSeconds` (+ DeltaSeconds (`self.CurrentLifetimeSeconds`))))
  (`SceneComponent.SetRelativeScale3D` (`self.DefaultSceneRoot`) _currentscale)
  (`/ArmorModules/Blueprints/Lib/PSM_Blueprint_Library.Shipping Safe Log` (`KismetStringLibrary.Concat_StrStr` "Currently scale " (`KismetStringLibrary.Conv_VectorToString` _currentscale) "  time " (`KismetStringLibrary.Conv_DoubleToString` _output_get)) "NewEnumerator3")
  (set `self.CurrentScale` (`KismetMathLibrary.VLerp` _currentscale (0.0 0.0 0.0) (`KismetMathLibrary.SafeDivide` (`self.CurrentLifetimeSeconds`) (`self.AnimationDurationSeconds`)))))

(fn `UserConstructionScript`)